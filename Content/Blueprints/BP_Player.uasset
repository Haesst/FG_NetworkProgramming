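; BP_Player is a player Blueprint that displays its local network role and rocket count through a WBP_Role widget held by the WidgetRole component.
; On BeginPlay it converts the local role enum to text and writes it to the widget.
; The OnNumRocketsChanged event passes each new count to SetNumRocketsInWidget, which casts the component's widget object and updates the displayed number.
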(event `self.ReceiveBeginPlay`
  (bind _aswbp_role (cast `/Game/Blueprints/UI/WBP_Role` (`WidgetComponent.GetUserWidgetObject` (`self.Widget_Role`))))
  (`/Game/Blueprints/UI/WBP_Role.SetLocalText` _aswbp_role (`KismetTextLibrary.Conv_StringToText` (`|GetEnumeratorNameAsString` (`self.GetLocalRole`)))))

(event `self.BP_OnNumRocketsChanged`
  (params (NewNumRockets :type Integer))
  (`self.SetNumRocketsInWidget` NewNumRockets))

(fn `SetNumRocketsInWidget`
  (params (InNumRockets :type Integer))
  (bind _aswbp_role (cast `/Game/Blueprints/UI/WBP_Role` (`WidgetComponent.GetUserWidgetObject` (`self.Widget_Role`))))
  (`/Game/Blueprints/UI/WBP_Role.SetNumRockets` _aswbp_role InNumRockets))

(fn `UserConstructionScript`)